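; Player tile for a grid-based board game that moves in steps, fires an optional upgrade and takes damage.
; A timeline lerps it one fixed step in the chosen direction, then notifies every BP_Tile that a movement was made, as also happens at BeginPlay.
; Damage is reduced by AttackStat and spawns an explosion, then either shows GameOver at zero health or increments EnemiesKilled.
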(event `MoveCharacter`
  (params (NewParam :type Integer))
  ;[1 1 1] Move the character.
  (bind _outactors (`GameplayStatics.GetAllActorsOfClass` "/Game/Blueprints/Tiles/BP_BoardTile.BP_BoardTile_C"))
  (set `self.BoardTilesRef` _outactors)
  (if (not (`TimelineComponent.IsPlaying` (`self.MovePawn`)))
    (set `self.LocationSaved` (`self.K2_GetActorLocation`))
    (bind (_direction _newtrack_0) (`Timeline|MovePawn` :!via `PlayFromStart`)
      (:`Update`
        (`self.K2_SetActorLocation` (`KismetMathLibrary.VLerp` (`self.LocationSaved`) (+ (`self.LocationSaved`) (select `int` NewParam :`0` (0.0 110.0 0.0) :`1` (0.0 -110.0 0.0) :`2` (110.0 0.0 0.0) :`3` (-110.0 0.0 0.0) :!type "Vector Structure")) _newtrack_0)))
      (:`Finished`
        ;[1 1 1] Tell every tile that a movement was made
        (bind _outactors_2 (`GameplayStatics.GetAllActorsOfClass` "/Game/Blueprints/Tiles/BP_Tile.BP_Tile_C" :!label _label))
        (for _array_element _outactors_2
          (`self.MovementWasMade` _array_element))))))

(event `self.ReceiveBeginPlay`
  ;[1 1 1] Bgin Play
  (`parent.ReceiveBeginPlay`)
  (goto _label))

(event `TryToFireTHeUpgrade`
  (params (TileThatIsFiring :type "/Game/Blueprints/Tiles/BP_Tile Object Reference"))
  (bind _myupgrade (`self.MyUpgrade`))
  (`/Engine/EditorBlueprintResources/StandardMacros.IsValid` _myupgrade
    (:`Is Valid`
      (`/Game/Blueprints/Upgrades/BP_UpgradeClass.Fire` _myupgrade TileThatIsFiring))))

(event `TakeDamage`
  (params (DamageValue :type "Float (double-precision)"))
  ;[1 1 1] Take damage and then Check if Game is Over
  (`GameplayStatics.SpawnEmitterAtLocation` "/Game/StarterContent/Particles/P_Explosion.P_Explosion" (`self.K2_GetActorLocation`))
  (bind _output_get (set `self.CurrentHealth` (- (`self.CurrentHealth`) (`KismetMathLibrary.FClamp` (- DamageValue (`self.AttackStat`)) 0.0 DamageValue))))
  (if (<= _output_get 0.0)
    (bind _returnvalue (`|CreateWidget` "/Game/Blueprints/UI/GameOver.GameOver_C"))
    (`UserWidget.AddToViewport` _returnvalue 0)
    (else
      (`/Engine/EditorBlueprintResources/StandardMacros.IncrementFloat` (`self.EnemiesKilled`)))))

(fn `UserConstructionScript`
  (`parent.UserConstructionScript`))