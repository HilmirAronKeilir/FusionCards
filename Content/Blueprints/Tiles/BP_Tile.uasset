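; BP_Tile is a board-game tile that serves as either a board cell or a content tile the player consumes by moving onto it.
; On BeginPlay it loads type, texture and value from Data_TileTypes, scaling nonzero values by squared enemy kills.
; After each move, upward traces let board cells refill with random tiles, while content tiles detect the player.
; Consumed tiles apply damage, healing, gold, death or an upgrade, unless the player's active upgrade intercepts.
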(event `self.ReceiveBeginPlay`
  (bind _textrender (`self.TextRender`))
  ;[1 1 1] Get Data about the tile and assign the correct texture and Values
  (bind _returnvalue (`|GetDataTableRow` "/Game/DataStuff/Data_TileTypes.Data_TileTypes" (`self.Type`))
    (:`then`
      (set `self.TileType` (`.ClassRef_6_9A8B8FD34E9A35AFDA4DA1AB12E85C03` (break `/Game/DataStuff/TileTypes` _returnvalue)))
      (if (== (`.DamageValue_9_A56F219F4C7A25D42DCE8FACEC404208` (break `/Game/DataStuff/TileTypes` _returnvalue)) 0.0)
        ;[1 1 1] Destroy the Text if the tile is just the board TIle
        (`ActorComponent.K2_DestroyComponent` _textrender)
        (else
          (bind _ascamera_pawn (cast `/Game/Blueprints/CameraPawn` (`GameplayStatics.GetPlayerPawn` 0)))
          (bind _enemieskilled (`/Game/Blueprints/Tiles/BP_PlayerTile.EnemiesKilled` (`/Game/Blueprints/CameraPawn.PlayerRef` _ascamera_pawn)))
          (bind _output_get (set `self.MyDamageType` (`KismetMathLibrary.Conv_IntToDouble` (`KismetMathLibrary.FFloor` (+ (* (* _enemieskilled _enemieskilled) (`.DamageMultiplier_21_3CEEECAF4EBF4DEFC42354888638BF5B` (break `/Game/DataStuff/TileTypes` _returnvalue))) (`.DamageValue_9_A56F219F4C7A25D42DCE8FACEC404208` (break `/Game/DataStuff/TileTypes` _returnvalue)))))))
          (`TextRenderComponent.K2_SetText` _textrender (`KismetTextLibrary.Conv_DoubleToText` _output_get "HalfToEven"))))
      (bind _returnvalue_2 (`PrimitiveComponent.CreateDynamicMaterialInstance` (`self.Plane`) 0 "/Game/Materials/mat_Background.mat_Background" "None"))
      (set `self.MyMaterialREf` _returnvalue_2)
      (`MaterialInstanceDynamic.SetTextureParameterValue` _returnvalue_2 "Texture" (break `/Game/DataStuff/TileTypes` _returnvalue))
      ;[1 1 1] Remove the Player from the Random TAble
      (bind _outrownames (`DataTableFunctionLibrary.GetDataTableRowNames` "/Game/DataStuff/Data_TileTypes.Data_TileTypes"))
      (set `self.RowsName` _outrownames)
      (`KismetArrayLibrary.Array_RemoveItem` (`self.RowsName`) "Player"))
    (:`RowNotFound`
      (`KismetSystemLibrary.PrintString` "ahhhhh"))))

(event `MovementWasMade`
  (bind _returnvalue (`self.K2_GetActorLocation`))
  (bind _returnvalue_2 (`self.K2_GetActorLocation`))
  ;[1 1 1] Do stuff when movement was Made
  (if (`self.IAmBoardTile`)
    ;[1 1 1] First see if I am empty and then try to spawn a random Tile
    (`KismetSystemLibrary.Delay` 0.1)
    (bind _outhit (`KismetSystemLibrary.LineTraceSingle` _returnvalue (+ _returnvalue (0.0 0.0 15.0)) "TraceTypeQuery1"))
    (cast `/Game/Blueprints/Tiles/BP_Tile` (`.HitActor` (`GameplayStatics.BreakHitResult` _outhit))
      (:`CastFailed`
        (`|SpawnActorFromClass` "/Game/Blueprints/Tiles/BP_TileEnemy.BP_TileEnemy_C" (`KismetMathLibrary.MakeTransform` (`self.K2_GetActorLocation`)) "Undefined" "OverrideRootScale" null (`KismetArrayLibrary.Array_Random` (`self.RowsName`)) "NewEnumerator0" null)))
    (else
      ;[1 1 1] See if player moved on top of me and then kill me
      (bind _outhit_2 (`KismetSystemLibrary.LineTraceSingle` (+ _returnvalue_2 (0.0 0.0 1.0)) (+ _returnvalue_2 (0.0 0.0 15.0)) "TraceTypeQuery1"))
      (bind _asbp_player_tile (cast `/Game/Blueprints/Tiles/BP_PlayerTile` (`.HitActor` (`GameplayStatics.BreakHitResult` _outhit_2))))
      (bind _myupgrade (`/Game/Blueprints/Tiles/BP_PlayerTile.MyUpgrade` _asbp_player_tile))
      (`/Engine/EditorBlueprintResources/StandardMacros.IsValid` _myupgrade
        (:`Is Valid`
          (`/Game/Blueprints/Upgrades/BP_UpgradeClass.Fire` _myupgrade self))
        (:`Is Not Valid`
          (`self.TileFunction` _asbp_player_tile :!label _label)
          (`self.K2_DestroyActor` :!label _label_2))))))

(event `DoFunction`
  (params (PlayerRef :type "/Game/Blueprints/Tiles/BP_PlayerTile Object Reference")))

(event `DoneFiring`
  (params (DoTheFunction :type Boolean))
  ;[1 1 1] See if player moved on top of me and then kill me
  (if DoTheFunction
    (goto _label)
    (else
      (goto _label_2))))

(fn `TileFunction`
  (params (PlayerRef :type "/Game/Blueprints/Tiles/BP_PlayerTile Object Reference"))
  (locals (NewLocalVar_0 :type "/Game/Blueprints/Tiles/BP_PlayerTile Object Reference"))
  (bind _newlocalvar_0 (`local.NewLocalVar_0`))
  (bind _newlocalvar_0_2 (`local.NewLocalVar_0`))
  (set `local.NewLocalVar_0` PlayerRef)
  (switch `/Game/FunctionTypes` (`self.TileType`)
    (:`NewEnumerator0`
      (`/Game/Blueprints/Tiles/BP_PlayerTile.TakeDamage` (`local.NewLocalVar_0`) (`self.MyDamageType`)))
    (:`NewEnumerator1`
      (set `/Game/Blueprints/Tiles/BP_PlayerTile.CurrentHealth` (`/Game/Blueprints/Tiles/BP_PlayerTile.MaxHealth` PlayerRef) (`local.NewLocalVar_0`)))
    (:`NewEnumerator2`
      (set `/Game/Blueprints/Tiles/BP_PlayerTile.Gold` (+ (`self.MyDamageType`) (`/Game/Blueprints/Tiles/BP_PlayerTile.Gold` _newlocalvar_0)) _newlocalvar_0))
    (:`NewEnumerator3`
      (set `/Game/Blueprints/Tiles/BP_PlayerTile.CurrentHealth` 0.0 _newlocalvar_0_2)
      (`/Game/Blueprints/Tiles/BP_PlayerTile.TakeDamage` _newlocalvar_0_2 0.0))
    (:`NewEnumerator4`
      (bind _returnvalue (`|GetDataTableRow` "/Game/DataStuff/Data_TileTypes.Data_TileTypes" (`self.Type`))
        (:`then`
          (bind _asbp_upgrade_class (castclass `/Game/Blueprints/Upgrades/BP_UpgradeClass` (`.UpgradeClass_11_BE8C21404C91EC3D949D6F844BD23F81` (break `/Game/DataStuff/UpgradeTypes` (`.UpgradeType_16_D47B6D014990935251D869958E06C885` (break `/Game/DataStuff/TileTypes` _returnvalue))))))
          (`|SpawnActorFromClass` _asbp_upgrade_class (`KismetMathLibrary.MakeTransform` (0.0 0.0 0.0)) "Undefined" "OverrideRootScale" null (`local.NewLocalVar_0`) null))))))

(fn `UserConstructionScript`)