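; Fusion upgrade actor that merges a monster tile into the player when fired.
; It looks up the firing tile's type in Data_TileTypes; for monsters, it copies the tile's texture to the player's Texture2 and sets Texture to MainFusion.
; Half the tile's MyDamageType is added to the player's AttackStat, computed before DoneFiring and applied after it.
; Non-monster tiles only finish firing with a debug print; both branches destroy the actor.
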(event `self.Fire`
  (params (TileThatIsFiring :type "/Game/Blueprints/Tiles/BP_Tile Object Reference"))
  (bind _mymaterialref (`/Game/Blueprints/Tiles/BP_Tile.MyMaterialREf` (`self.PlayerRef`)))
  (set `self.FiringTile` TileThatIsFiring)
  (bind _returnvalue (`|GetDataTableRow` "/Game/DataStuff/Data_TileTypes.Data_TileTypes" (`/Game/Blueprints/Tiles/BP_Tile.Type` TileThatIsFiring))
    (:`then`
      (if (`.IsMonster_18_016C89EB4E1702A198127CAC49A85DCD` (break `/Game/DataStuff/TileTypes` _returnvalue))
        (bind _returnvalue_2 (`MaterialInstanceDynamic.K2_GetTextureParameterValue` (`/Game/Blueprints/Tiles/BP_Tile.MyMaterialREf` (`self.FiringTile`)) "Texture"))
        (`MaterialInstanceDynamic.SetTextureParameterValue` _mymaterialref "Texture2" _returnvalue_2)
        (`MaterialInstanceDynamic.SetTextureParameterValue` _mymaterialref "Texture" "/Game/Blueprints/Tiles/mainFusion.mainFusion")
        (set `self.SavedAttackStat` (+ (/ (`/Game/Blueprints/Tiles/BP_Tile.MyDamageType` (`self.FiringTile`)) 2.0) (`/Game/Blueprints/Tiles/BP_PlayerTile.AttackStat` (`self.PlayerRef`))))
        (`/Game/Blueprints/Tiles/BP_Tile.DoneFiring` (`self.FiringTile`) true)
        (set `/Game/Blueprints/Tiles/BP_PlayerTile.AttackStat` (`self.SavedAttackStat`) (`self.PlayerRef`))
        (`self.K2_DestroyActor`)
        (else
          (`/Game/Blueprints/Tiles/BP_Tile.DoneFiring` (`self.FiringTile`) true)
          (`KismetSystemLibrary.PrintString` "not monster")
          (`self.K2_DestroyActor`))))))

(event `self.ReceiveBeginPlay`
  (`parent.ReceiveBeginPlay`))

(fn `UserConstructionScript`
  (`parent.UserConstructionScript`))