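; CameraPawn is the input pawn for a tile-board game, spawning the player tile and relaying movement to it.
; On BeginPlay it spawns BP_PlayerTile, caches all BP_BoardTile actors and adds a Stats widget linked to the player to the viewport.
; Four directional input actions call MoveCharacter on the tile, unless its location is within tolerance of that side's hard-coded board edge.
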(event `self.ReceiveBeginPlay`
  ;[1 1 1] Comment
  (bind _returnvalue (`|SpawnActorFromClass` "/Game/Blueprints/Tiles/BP_PlayerTile.BP_PlayerTile_C" (`KismetMathLibrary.MakeTransform` (-110.0 110.0 5.0)) "Undefined" "OverrideRootScale" null "Player" "NewEnumerator0" null))
  (set `self.PlayerRef` _returnvalue)
  (bind _outactors (`GameplayStatics.GetAllActorsOfClass` "/Game/Blueprints/Tiles/BP_BoardTile.BP_BoardTile_C"))
  (set `self.TilesRef` _outactors)
  (bind _returnvalue_2 (`|CreateWidget` "/Game/Blueprints/UI/Stats.Stats_C" null (`self.PlayerRef`)))
  (`UserWidget.AddToViewport` _returnvalue_2 0)
  (set `self.StatScreenRef` _returnvalue_2))

(event `InputAction|MoveLeft`
  (params (Key :type "Key Structure"))
  (bind (_returnvalue_x _returnvalue_y) (`KismetMathLibrary.BreakVector` (`self.K2_GetActorLocation` (`self.PlayerRef`))))
  ;[1 1 1] Movements
  (:`Pressed`
    (if (not (`KismetMathLibrary.NearlyEqual_FloatFloat` _returnvalue_y 0.0 10.0))
      (`/Game/Blueprints/Tiles/BP_PlayerTile.MoveCharacter` (`self.PlayerRef`) 1))))

(event `InputAction|MoveRight`
  (params (Key :type "Key Structure"))
  (bind (_returnvalue_x _returnvalue_y) (`KismetMathLibrary.BreakVector` (`self.K2_GetActorLocation` (`self.PlayerRef`))))
  ;[1 1 1] Movements
  (:`Pressed`
    (if (not (`KismetMathLibrary.NearlyEqual_FloatFloat` _returnvalue_y 220.0 10.0))
      (`/Game/Blueprints/Tiles/BP_PlayerTile.MoveCharacter` (`self.PlayerRef`) 0))))

(event `InputAction|MoveUp`
  (params (Key :type "Key Structure"))
  (bind _returnvalue_x (`KismetMathLibrary.BreakVector` (`self.K2_GetActorLocation` (`self.PlayerRef`))))
  ;[1 1 1] Movements
  (:`Pressed`
    (if (not (`KismetMathLibrary.NearlyEqual_FloatFloat` _returnvalue_x 0.0 10.0))
      (`/Game/Blueprints/Tiles/BP_PlayerTile.MoveCharacter` (`self.PlayerRef`) 2))))

(event `InputAction|MoveDown`
  (params (Key :type "Key Structure"))
  (bind _returnvalue_x (`KismetMathLibrary.BreakVector` (`self.K2_GetActorLocation` (`self.PlayerRef`))))
  ;[1 1 1] Movements
  (:`Pressed`
    (if (not (`KismetMathLibrary.NearlyEqual_FloatFloat` _returnvalue_x -220.0 10.0))
      (`/Game/Blueprints/Tiles/BP_PlayerTile.MoveCharacter` (`self.PlayerRef`) 3))))

(fn `UserConstructionScript`)